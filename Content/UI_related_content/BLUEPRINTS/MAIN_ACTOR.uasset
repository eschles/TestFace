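; Main actor that displays the player's customized character on its UIHEAD skeletal mesh, apparently for the customization UI.
; On BeginPlay it reads gender, business or casual outfit, skin tint and age from the PlayerCustomization_INST game instance.
; ChangeMesh swaps skeletal mesh, per-slot materials and anim class for each of four body variants, then skin tint and age drive the TintScalar and Oldness material parameters.
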(event `self.ReceiveBeginPlay`
  (bind _ui_head (`self.UI_HEAD`))
  ;[1 1 1] Main_Actor
  (bind _asplayer_customization_inst (cast `/Game/GameInstances/PlayerCustomization_INST` (`GameplayStatics.GetGameInstance`)))
  (if (`/Game/GameInstances/PlayerCustomization_INST.genderFemale` _asplayer_customization_inst)
    (`self.ChangeMesh` "NewEnumerator2")
    (bind _business (`/Game/GameInstances/PlayerCustomization_INST.business` _asplayer_customization_inst))
    (if (not _business)
      (`self.ChangeMesh` "NewEnumerator3"))
    (bind _skintint (`/Game/GameInstances/PlayerCustomization_INST.skinTint` _asplayer_customization_inst))
    (`MeshComponent.SetScalarParameterValueOnMaterials` _ui_head "TintScalar" _skintint)
    (bind _age (`/Game/GameInstances/PlayerCustomization_INST.age` _asplayer_customization_inst))
    (`MeshComponent.SetScalarParameterValueOnMaterials` _ui_head "Oldness" _age)
    (else
      (`self.ChangeMesh` "NewEnumerator0")
      (if (not _business)
        (`self.ChangeMesh` "NewEnumerator1"))
      (`MeshComponent.SetScalarParameterValueOnMaterials` _ui_head "TintScalar" _skintint)
      (`MeshComponent.SetScalarParameterValueOnMaterials` _ui_head "Oldness" _age))))

(fn `ChangeMesh`
  (params (NewParam :type "/Game/UI_related_content/BLUEPRINTS/EBodyTypes Enum" :default "NewEnumerator0"))
  (switch `/Game/UI_related_content/BLUEPRINTS/EBodyTypes` NewParam
    (:`NewEnumerator0`
      (`SkinnedMeshComponent.SetSkinnedAssetAndUpdate` (`self.UI_HEAD`) "/Game/Models/BaseMale/SecondRigTest/Body2.Body2" true)
      (`self.SetMaleBusinessMaterials`)
      (`SkeletalMeshComponent.SetAnimInstanceClass` (`self.UI_HEAD`) "/Game/Animations/MaleBusiness/MaleBusiness_AnimBlueprint.MaleBusiness_AnimBlueprint_C"))
    (:`NewEnumerator1`
      (`SkinnedMeshComponent.SetSkinnedAssetAndUpdate` (`self.UI_HEAD`) "/Game/Models/CasualMale/CasualMale.CasualMale" true)
      (`self.SetMaleCasualMaterials`)
      (`SkeletalMeshComponent.SetAnimInstanceClass` (`self.UI_HEAD`) "/Game/Animations/MaleCasual/MaleCasual_AnimBlueprint.MaleCasual_AnimBlueprint_C"))
    (:`NewEnumerator2`
      (`SkinnedMeshComponent.SetSkinnedAssetAndUpdate` (`self.UI_HEAD`) "/Game/Models/BusinessFemale/FemaleBusiness.FemaleBusiness" true)
      (`self.SetFemaleBusinessMaterials`)
      (`SkeletalMeshComponent.SetAnimInstanceClass` (`self.UI_HEAD`) "/Game/Animations/FemaleBusiness/FemaleBusiness_AnimBlueprint.FemaleBusiness_AnimBlueprint_C"))
    (:`NewEnumerator3`
      (`SkinnedMeshComponent.SetSkinnedAssetAndUpdate` (`self.UI_HEAD`) "/Game/Models/CasualFemale/CasualFemale.CasualFemale" true)
      (`self.SetFemaleCasualMaterials`)
      (`SkeletalMeshComponent.SetAnimInstanceClass` (`self.UI_HEAD`) "/Game/Animations/FemaleCasual/FemaleCasual_AnimBlueprint.FemaleCasual_AnimBlueprint_C"))))

(fn `SetFemaleBusinessMaterials`
  (bind _ui_head (`self.UI_HEAD`))
  (`PrimitiveComponent.SetMaterial` _ui_head 0 "/Game/Materials/FemaleSkin/FemaleHair_MAT.FemaleHair_MAT")
  (`PrimitiveComponent.SetMaterial` _ui_head 1 "/Game/Materials/EyeMaterials/Right_Eye_Inst.Right_Eye_Inst")
  (`PrimitiveComponent.SetMaterial` _ui_head 2 "/Game/Materials/EyeMaterials/Left_Eye_Inst.Left_Eye_Inst")
  (`PrimitiveComponent.SetMaterial` _ui_head 3 "/Game/Materials/FemaleSkin/Business/FemaleBusiness_MAT_Inst.FemaleBusiness_MAT_Inst")
  (`PrimitiveComponent.SetMaterial` _ui_head 4 "/Game/Materials/FemaleSkin/Business/FemaleBusiness_MAT_Inst.FemaleBusiness_MAT_Inst")
  (`PrimitiveComponent.SetMaterial` _ui_head 5 "/Game/Materials/FemaleSkin/FemaleHead_MAT_Inst.FemaleHead_MAT_Inst"))

(fn `SetFemaleCasualMaterials`
  (bind _ui_head (`self.UI_HEAD`))
  (`PrimitiveComponent.SetMaterial` _ui_head 0 "/Game/Materials/FemaleSkin/FemaleHair_MAT.FemaleHair_MAT")
  (`PrimitiveComponent.SetMaterial` _ui_head 1 "/Game/Materials/EyeMaterials/Right_Eye_Inst.Right_Eye_Inst")
  (`PrimitiveComponent.SetMaterial` _ui_head 2 "/Game/Materials/EyeMaterials/Left_Eye_Inst.Left_Eye_Inst")
  (`PrimitiveComponent.SetMaterial` _ui_head 3 "/Game/Materials/FemaleSkin/Casual/FemaleCasual_MAT_Inst.FemaleCasual_MAT_Inst")
  (`PrimitiveComponent.SetMaterial` _ui_head 4 "/Game/Materials/FemaleSkin/Casual/FemaleCasual_MAT_Inst.FemaleCasual_MAT_Inst")
  (`PrimitiveComponent.SetMaterial` _ui_head 5 "/Game/Materials/FemaleSkin/FemaleHead_MAT_Inst.FemaleHead_MAT_Inst"))

(fn `SetMaleBusinessMaterials`
  (bind _ui_head (`self.UI_HEAD`))
  (`PrimitiveComponent.SetMaterial` _ui_head 0 "/Game/Materials/MaleSkin/TestHead1_MAT_Inst.TestHead1_MAT_Inst")
  (`PrimitiveComponent.SetMaterial` _ui_head 1 "/Game/Models/BaseMale/mouth.mouth")
  (`PrimitiveComponent.SetMaterial` _ui_head 2 "/Game/Materials/EyeMaterials/Left_Eye_Inst.Left_Eye_Inst")
  (`PrimitiveComponent.SetMaterial` _ui_head 3 "/Game/UI_related_content/MATERIALS/OFF-WHITE_MAT.OFF-WHITE_MAT")
  (`PrimitiveComponent.SetMaterial` _ui_head 4 "/Game/UI_related_content/MATERIALS/BLACK_MAT.BLACK_MAT")
  (`PrimitiveComponent.SetMaterial` _ui_head 5 "/Game/UI_related_content/MATERIALS/BLACK_MAT.BLACK_MAT")
  (`PrimitiveComponent.SetMaterial` _ui_head 6 "/Game/UI_related_content/MATERIALS/BLACK_MAT.BLACK_MAT"))

(fn `SetMaleCasualMaterials`
  (bind _ui_head (`self.UI_HEAD`))
  (`PrimitiveComponent.SetMaterial` _ui_head 0 "/Game/Materials/MaleSkin/TestHead1_MAT_Inst.TestHead1_MAT_Inst")
  (`PrimitiveComponent.SetMaterial` _ui_head 1 "/Game/Materials/EyeMaterials/Right_Eye_Inst.Right_Eye_Inst")
  (`PrimitiveComponent.SetMaterial` _ui_head 2 "/Game/Materials/EyeMaterials/Left_Eye_Inst.Left_Eye_Inst")
  (`PrimitiveComponent.SetMaterial` _ui_head 3 "/Game/Materials/FemaleSkin/Casual/FemaleCasual_MAT_Inst.FemaleCasual_MAT_Inst")
  (`PrimitiveComponent.SetMaterial` _ui_head 4 "/Game/Materials/MaleSkin/MaleHair_MAT.MaleHair_MAT"))

(fn `UserConstructionScript`
  (`KismetMaterialLibrary.CreateDynamicMaterialInstance` "/Game/UI_related_content/MATERIALS/MultiColor_Shirt_INST.MultiColor_Shirt_INST")
  (`KismetMaterialLibrary.CreateDynamicMaterialInstance` "/Game/Materials/MaleSkin/TestHead1_MAT_Inst.TestHead1_MAT_Inst"))