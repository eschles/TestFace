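; Test actor that previews every morph target on a skeletal mesh by animating them one after another.
; BeginPlay caches the mesh's morph target names and their count.
; Each Tick derives the active target from game time and MorphTestSpeed, eases its weight from zero to one and back on a cosine curve, and prints its name.
; Each cosine period advances to the next target, looping through the list.
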(event `self.ReceiveBeginPlay`
  (bind _output_get (set `self.MorphTargets` (`SkeletalMesh.K2_GetAllMorphTargetNames` (`SkinnedMeshComponent.SkeletalMesh` (`self.SkeletalMesh`)))))
  (set `self.MorphCount` (`KismetArrayLibrary.Array_Length` _output_get)))

(event `self.ReceiveTick`
  (params (DeltaSeconds :type "Float (single-precision)"))
  (bind _returnvalue (* (`GameplayStatics.GetTimeSeconds`) (`self.MorphTestSpeed`)))
  (bind _output (`|GetArrayItem` (`self.MorphTargets`) (`KismetMathLibrary.FFloor` (mod (/ _returnvalue (`KismetMathLibrary.MultiplyByPi` 2.0)) (`KismetMathLibrary.Conv_IntToDouble` (`self.MorphCount`))))))
  (`SkeletalMeshComponent.SetMorphTarget` (`self.SkeletalMesh`) (`KismetStringLibrary.Conv_StringToName` _output) (/ (- 1.0 (`KismetMathLibrary.Cos` _returnvalue)) 2.0) true)
  (`KismetSystemLibrary.PrintString` _output))

(fn `NewFunction_0`)

(fn `UserConstructionScript`)